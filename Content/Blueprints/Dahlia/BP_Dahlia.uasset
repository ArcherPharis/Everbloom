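; Dahlia character Blueprint that handles her death sequence and a time-freeze ability.
; Death slows global time, fades the camera and opens the title screen.
; TimeFreeze zeroes every Emilia actor's custom time dilation while a timeline animates a material parameter collection, then sends a delayed gameplay event to signal the freeze's stop.
; TimeFreezeEnd restores those actors' time and drives the material scalars from a second timeline.
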(event Custom|TimeFreeze
  (Utilities|FlowControl|Sequence
    (:then_0
      (bind _alpha (Timeline|Timeline PlayFromStart)
        (:Update
          (Rendering|Material|SetScalarParameterValue "/Game/Blueprints/GAS/Abilities/Magic/Freeze/MPC_TimeFreeze.MPC_TimeFreeze" "Scalar" _alpha :!class /Script/Engine.KismetMaterialLibrary)
          (Rendering|Material|SetVectorParameterValue "/Game/Blueprints/GAS/Abilities/Magic/Freeze/MPC_TimeFreeze.MPC_TimeFreeze" "Vector" (Math|Color|Lerp(LinearColor) "(R=0.000000,G=0.473850,B=1.000000,A=1.000000)" "(R=0.000000,G=0.849591,B=1.000000,A=1.000000)" _alpha) :!class /Script/Engine.KismetMaterialLibrary)
          (if (>= _alpha 1.6)
            (Rendering|Material|SetScalarParameterValue "/Game/Blueprints/GAS/Abilities/Magic/Freeze/MPC_TimeFreeze.MPC_TimeFreeze" "Scalar1" 1.0 :!class /Script/Engine.KismetMaterialLibrary)
            (Utilities|FlowControl|Delay 4.0)
            (Ability|SendGameplayEventtoActor self "(TagName=\"Abilities.Main.Freeze.Stop\")")))))
    (:then_1
      (bind _outactors (Actor|GetAllActorsOfClass "/Script/Everbloom.Emilia"))
      (for _array_element _outactors
        (Variables|/Script/Engine.Actor|SetCustomTimeDilation _array_element 0.0)))))

(event Custom|TimeFreezeEnd
  (Utilities|FlowControl|Sequence
    (:then_0
      (bind _alpha (Timeline|Timeline_0 PlayFromStart)
        (:Update
          (Rendering|Material|SetScalarParameterValue "/Game/Blueprints/GAS/Abilities/Magic/Freeze/MPC_TimeFreeze.MPC_TimeFreeze" "Scalar" _alpha :!class /Script/Engine.KismetMaterialLibrary)
          (Rendering|Material|SetScalarParameterValue "/Game/Blueprints/GAS/Abilities/Magic/Freeze/MPC_TimeFreeze.MPC_TimeFreeze" "Scalar1" _alpha :!class /Script/Engine.KismetMaterialLibrary))))
    (:then_1
      (bind _outactors (Actor|GetAllActorsOfClass "/Script/Everbloom.Emilia"))
      (for _array_element _outactors
        (Variables|/Script/Engine.Actor|SetCustomTimeDilation _array_element 1.0)))))

(event EventBeginPlay)

(event Collision|EventActorBeginOverlap
  (params (OtherActor :type Actor%20Object%20Reference)))

(event EventTick
  (params (DeltaSeconds :type Float%20%28single-precision%29)))

(event EventOnDahliaDeath
  (Utilities|Time|SetGlobalTimeDilation 0.5)
  (CameraFades|StartCameraFade :self (Game|GetPlayerCameraManager 0) :ToAlpha 1.0 :Duration 6.0)
  (Utilities|FlowControl|Delay 6.0)
  (Game|OpenLevel(byName) "TitleScreen"))

(fn ConstructionScript)