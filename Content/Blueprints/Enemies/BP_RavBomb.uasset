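; BP_RavBomb is an enemy bomb actor that explodes after a random delay between its min and max detonate times.
; On detonation it spawns a scaled-up explosion emitter, applies GE_BombEffect through the Ability System to characters overlapping its Sphere, then plays a sound and destroys itself.
; The cast inside the overlap loop has no failure branch, so non-BaseCharacter actors receive no effect.
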(event EventBeginPlay
  (Utilities|FlowControl|Delay (Math|Random|RandomFloatinRange (Variables|Default|GetMinDentonateTime) (Variables|Default|GetMaxDentonate%20Time)))
  (Effects|SpawnEmitteratLocation "/Game/SmokeFX/Particles/P_ExplosionBig_01.P_ExplosionBig_01" (Transformation|GetActorLocation) "0, 0, 0" "5.000000,5.000000,5.000000")
  (for _array_element (Collision|GetOverlappingActors (Variables|Default|GetSphere) 0 :!class /Script/Engine.PrimitiveComponent)
    (bind _asbase_character (Utilities|Casting|CastToBaseCharacter _array_element))
    (GameplayEffects|ApplyGameplayEffectToSelf :self (Ability|GetAbilitySystemComponent _asbase_character) :GameplayEffectClass "/Game/Blueprints/Enemies/GE_BombEffect.GE_BombEffect_C"))
  (Audio|PlaySoundatLocation "/Game/StarterContent/Audio/Explosion_Cue.Explosion_Cue" (Transformation|GetActorLocation) "0, 0, 0" 1.0 1.0 0.0 0 0 0 0)
  (Actor|DestroyActor))

(event Collision|EventActorBeginOverlap
  (params (OtherActor :type Actor%20Object%20Reference)))

(event EventTick
  (params (DeltaSeconds :type Float%20%28single-precision%29)))

(fn ConstructionScript)