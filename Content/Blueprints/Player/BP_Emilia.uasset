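; Player character Emilia, hosting the world-side effects of a Time Freeze ability and debug keys that self-apply Thunderbolt and test-heal gameplay effects.
; TimeFreeze locks input during its intro timeline, animates a Material Parameter Collection and zeroes every BaseEnemy's CustomTimeDilation.
; After a delay it sends a GAS stop event; TimeFreezeEnd restores enemy time and animates the visuals out.
; Also hides the weapon bone and timeline-rotates toward targets.
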(event Custom|TimeFreeze
  (Utilities|FlowControl|Sequence
    (:then_0
      (bind _asplayer_controller (Utilities|Casting|CastToPlayerController (Components|GetOwner)))
      (Input|DisableInput _asplayer_controller)
      (bind _alpha (Timeline|TFTimeline PlayFromStart)
        (:Update
          (Rendering|Material|SetScalarParameterValue "/Game/Blueprints/GAS/Abilities/Magic/Freeze/MPC_TimeFreeze.MPC_TimeFreeze" "Scalar" _alpha :!class /Script/Engine.KismetMaterialLibrary)
          (Rendering|Material|SetVectorParameterValue "/Game/Blueprints/GAS/Abilities/Magic/Freeze/MPC_TimeFreeze.MPC_TimeFreeze" "Vector" (Math|Color|Lerp(LinearColor) "(R=0.000000,G=0.473850,B=1.000000,A=1.000000)" "(R=0.000000,G=0.849591,B=1.000000,A=1.000000)" _alpha) :!class /Script/Engine.KismetMaterialLibrary)
          (if (>= _alpha 1.6)
            (Rendering|Material|SetScalarParameterValue "/Game/Blueprints/GAS/Abilities/Magic/Freeze/MPC_TimeFreeze.MPC_TimeFreeze" "Scalar1" 1.0 :!class /Script/Engine.KismetMaterialLibrary)
            (Utilities|FlowControl|Delay (Variables|Default|GetTimeFreeze%20Duration))
            (Ability|SendGameplayEventtoActor self "(TagName=\"Abilities.Main.Freeze.Stop\")")))
        (:Finished
          (Input|EnableInput _asplayer_controller))))
    (:then_1
      (bind _outactors (Actor|GetAllActorsOfClass "/Script/Everbloom.BaseEnemy"))
      (for _array_element _outactors
        (Variables|/Script/Engine.Actor|SetCustomTimeDilation _array_element 0.0)))))

(event Custom|TimeFreezeEnd
  (Utilities|FlowControl|Sequence
    (:then_0
      (bind _alpha (Timeline|TFETimeline PlayFromStart)
        (:Update
          (Rendering|Material|SetScalarParameterValue "/Game/Blueprints/GAS/Abilities/Magic/Freeze/MPC_TimeFreeze.MPC_TimeFreeze" "Scalar" _alpha :!class /Script/Engine.KismetMaterialLibrary)
          (Rendering|Material|SetScalarParameterValue "/Game/Blueprints/GAS/Abilities/Magic/Freeze/MPC_TimeFreeze.MPC_TimeFreeze" "Scalar1" _alpha :!class /Script/Engine.KismetMaterialLibrary))))
    (:then_1
      (bind _outactors (Actor|GetAllActorsOfClass "/Script/Everbloom.BaseEnemy"))
      (for _array_element _outactors
        (Variables|/Script/Engine.Actor|SetCustomTimeDilation _array_element 1.0)))))

(event EventBeginPlay
  (Components|SkinnedMesh|HideBonebyName (Variables|Character|GetMesh) "weapon" "PBO_None"))

(event Collision|EventActorBeginOverlap
  (params (OtherActor :type Actor%20Object%20Reference)))

(event EventTick
  (params (DeltaSeconds :type Float%20%28single-precision%29)))

(event EventRotatetoTargetEvent
  (params (Target :type Actor%20Object%20Reference))
  (bind _alpha (Timeline|RotateTimeline Play)
    (:Update
      (Transformation|SetActorRotation (Math|Rotator|MakeRotator (.roll (Math|Rotator|Lerp(Rotator) (Transformation|GetActorRotation) (Math|Rotator|FindLookatRotation (Transformation|GetActorLocation) (Transformation|GetActorLocation Target)) _alpha)) 0.0 (.yaw (Math|Rotator|Lerp(Rotator) (Transformation|GetActorRotation) (Math|Rotator|FindLookatRotation (Transformation|GetActorLocation) (Transformation|GetActorLocation Target)) _alpha)))))))

(event Input|KeyboardEvents|H
  (params (Key :type Key%20Structure :default "None"))
  (:Pressed
    (GameplayEffects|ApplyGameplayEffectToSelf :self (Ability|GetAbilitySystemComponent self) :GameplayEffectClass "/Game/Blueprints/GAS/Abilities/Magic/TBolt/BP_GE_Thunderbolt.BP_GE_Thunderbolt_C")))

(event Input|KeyboardEvents|G
  (params (Key :type Key%20Structure :default "None"))
  (:Pressed
    (GameplayEffects|ApplyGameplayEffectToSelf :self (Ability|GetAbilitySystemComponent self) :GameplayEffectClass "/Game/Blueprints/GAS/Abilities/Magic/TBolt/BP_GE_TestHeal.BP_GE_TestHeal_C")))

(fn ConstructionScript)