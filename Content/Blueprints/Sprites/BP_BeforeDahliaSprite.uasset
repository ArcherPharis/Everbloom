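; BP_BeforeDahliaSprite is an interactable blocker that turns Emilia back when she enters its Stopper volume.
; On overlap, it fades the camera in from full opacity, moves and rotates BP_Emilia to EmiliaTeleportLocation, then calls her Interact with itself as the target.
; The OnRemoveBlocker event destroys the Stopper component, which permanently opens the way.
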(event OnComponentBeginOverlap(Stopper)
  (params (OverlappedComponent :type Primitive%20Component%20Object%20Reference) (OtherActor :type Actor%20Object%20Reference) (OtherComp :type Primitive%20Component%20Object%20Reference) (OtherBodyIndex :type Integer) (bFromSweep :type Boolean) (SweepResult :type Hit%20Result%20Structure%20%28by%20ref%29))
  (bind _emiliateleportlocation (Variables|Default|GetEmiliaTeleportLocation))
  (bind _output_get (Variables|Default|SetOther%20Actor OtherActor))
  (if (== (Utilities|GetClass _output_get) "/Game/Blueprints/Player/BP_Emilia.BP_Emilia_C")
    (bind _asbp_emilia (Utilities|Casting|CastToBP_Emilia _output_get))
    (CameraFades|StartCameraFade :self (Game|GetPlayerCameraManager 0) :FromAlpha 1.0 :Duration 3.0)
    (Transformation|SetActorLocation _asbp_emilia (Transformation|GetWorldLocation _emiliateleportlocation) false false)
    (Transformation|SetActorRotation _asbp_emilia (Transformation|GetWorldRotation _emiliateleportlocation))
    (Class|Emilia|Interact _asbp_emilia self)))

(event EventBeginPlay)

(event Collision|EventActorBeginOverlap
  (params (OtherActor :type Actor%20Object%20Reference)))

(event EventTick
  (params (DeltaSeconds :type Float%20%28single-precision%29)))

(event EventOnRemoveBlocker
  (Components|DestroyComponent (Variables|Default|GetStopper)))

(fn ConstructionScript)