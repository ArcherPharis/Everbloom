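; Gameplay Ability for blocking that punishes a blocked attacker with a slow-motion knockback.
; OnBlock spawns a Niagara blink at the avatar, plays a slash sound at world origin, and briefly slows global time before launching the attacking Character along the avatar's forward vector.
; OnEndAbility restores normal time and applies GE_RemoveBlockStatus to the owner.
; ActivateAbility is unimplemented in this graph.
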(event Ability|EventActivateAbility)

(event Ability|EventOnEndAbility
  (params (bWasCancelled :type Boolean))
  (Utilities|Time|SetGlobalTimeDilation 1.0)
  (GameplayEffects|ApplyGameplayEffectToSelf :self (Ability|GetAbilitySystemComponentfromActorInfo) :GameplayEffectClass "/Game/Blueprints/GAS/Abilities/Block/GE_RemoveBlockStatus.GE_RemoveBlockStatus_C"))

(event EventOnBlock
  (params (Attacker :type Actor%20Object%20Reference))
  (bind _returnvalue (Class|EBGameplayAbilityBase|GetAvatarasCharacter))
  (bind _ascharacter (Utilities|Casting|CastToCharacter Attacker))
  (Niagara|SpawnSystematLocation "/Game/BlinkAndDashVFX/VFX_Niagara/NS_Blink_Psionic.NS_Blink_Psionic" (Transformation|GetActorLocation _returnvalue) (Transformation|GetActorRotation _returnvalue))
  (Audio|PlaySoundatLocation "/Game/Audio/Sword_Slash_1_v1.Sword_Slash_1_v1" "0, 0, 0" "0, 0, 0" 1.0 1.0 0.0 0 0 0 0)
  (Utilities|Time|SetGlobalTimeDilation 0.5)
  (Utilities|FlowControl|Delay 0.2)
  (Utilities|Time|SetGlobalTimeDilation 1.0)
  (Character|LaunchCharacter _ascharacter (* (Transformation|GetActorForwardVector (Class|EBGameplayAbilityBase|GetAvatarasCharacter)) 1.5e+03) false false))