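; BP_FireProjectile is a Fireburst magic ability projectile that handles its damage response through ApplyDamageEffect.
; If the caster has an Ability System Component, it applies a gameplay effect to the damaged actor, spawns impact Niagara and sound there, then destroys itself.
; Despite the fire name, it uses GE_GustDamage, a green lightning impact and a wind sound.
; Movement and hit detection are absent from these graphs.
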(event EventBeginPlay
  (|CallParentFunction) ; This node is disabled and will not be called.\nDrag off pins to build functionality.
)

(event Collision|EventActorBeginOverlap
  (params (OtherActor :type Actor%20Object%20Reference))
  (|CallParentFunction OtherActor) ; This node is disabled and will not be called.\nDrag off pins to build functionality.
)

(event EventTick
  (params (DeltaSeconds :type Float%20%28single-precision%29))
  (|CallParentFunction DeltaSeconds) ; This node is disabled and will not be called.\nDrag off pins to build functionality.
)

(event EventApplyDamageEffect
  (params (Caster :type Actor%20Object%20Reference) (Damaged :type Actor%20Object%20Reference))
  (bind _returnvalue (Ability|GetAbilitySystemComponent Caster))
  (bind _returnvalue_2 (Transformation|GetActorLocation Damaged))
  (Utilities|IsValid _returnvalue
    (:Is%20Valid
      (GameplayEffects|ApplyGameplayEffectToTarget :self _returnvalue :GameplayEffectClass "/Game/Blueprints/GAS/Abilities/Magic/Gust/AimVersion/GE_GustDamage.GE_GustDamage_C" :Target (Ability|GetAbilitySystemComponent Damaged))
      (Niagara|SpawnSystematLocation "/Game/Magic_Projectiles/MagicProjectiles_Optimal/Niagara/Lightning/NS_Lightning_Impact_Green_Fix.NS_Lightning_Impact_Green_Fix" _returnvalue_2)
      (Audio|SpawnSoundatLocation "/Game/Audio/Emilia/Wind/Emilia_WindImpact.Emilia_WindImpact" _returnvalue_2 "0, 0, 0" 1.0 1.0 0.0 0 0)
      (Actor|DestroyActor))))

(fn ConstructionScript
  (|CallParentFunction))