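; Point light actor for the Celes anime shader that registers itself with AC_CelesLightReceive components on actors within its attenuation radius.
; A radius trace filtered by object type and tag registers receivers at BeginPlay and, for editor preview, at construction.
; A radius-matched sphere registers tagged actors entering and deregisters those leaving.
; Interface getters expose the light and its intensity, smoothstep and filter data, while EnableOriginLight sets the real light's visibility.
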(event OnComponentBeginOverlap(SphereVolume)
  (params (OverlappedComponent :type Primitive%20Component%20Object%20Reference) (OtherActor :type Actor%20Object%20Reference) (OtherComp :type Primitive%20Component%20Object%20Reference) (OtherBodyIndex :type Integer) (bFromSweep :type Boolean) (SweepResult :type Hit%20Result%20Structure%20%28by%20ref%29))
  (bind _returnvalue (Actor|GetComponentbyClass OtherActor "/Game/CelesAnimeShader/BP/CelesLight/AC_CelesLightReceive.AC_CelesLightReceive_C"))
  (Utilities|IsValid _returnvalue
    (:Is%20Valid
      (bind _array_element (Utilities|Array|ForEachLoopwithBreak (Variables|/Script/Engine.Actor|GetTags OtherActor) :!label _label)
        (:LoopBody
          (if (Utilities|Array|ContainsItem (Variables|CelesLight|GetCelesLightFilterActorTag) _array_element)
            (Default|RegistLight _returnvalue self false)
            (goto _label Break)))))))

(event OnComponentEndOverlap(SphereVolume)
  (params (OverlappedComponent :type Primitive%20Component%20Object%20Reference) (OtherActor :type Actor%20Object%20Reference) (OtherComp :type Primitive%20Component%20Object%20Reference) (OtherBodyIndex :type Integer))
  (bind _returnvalue (Actor|GetComponentbyClass OtherActor "/Game/CelesAnimeShader/BP/CelesLight/AC_CelesLightReceive.AC_CelesLightReceive_C"))
  (Utilities|IsValid _returnvalue
    (:Is%20Valid
      (Default|DeregistLight _returnvalue self false))))

(event EventBeginPlay
  (bind _receiveactors (CallFunction|CelesLightReceiveTrace self (Transformation|GetActorLocation) (Variables|CelesLight|GetCelesLightEffectObjectType) (Variables|CelesLight|GetCelesLightFilterActorTag) (Variables|/Script/Engine.LocalLightComponent|GetAttenuationRadius (Variables|Default|GetPointLightComponent))))
  (for _array_element _receiveactors
    (Utilities|IsValid (Actor|GetComponentbyClass _array_element "/Game/CelesAnimeShader/BP/CelesLight/AC_CelesLightReceive.AC_CelesLightReceive_C")
      (:Is%20Valid
        (Default|RegistLight (Actor|GetComponentbyClass _array_element "/Game/CelesAnimeShader/BP/CelesLight/AC_CelesLightReceive.AC_CelesLightReceive_C") self false)))))

(fn ConstructionScript
  (CallFunction|ConstructionUpdate))

(fn ConstructionUpdate
  (bind _spherevolume (Variables|Default|GetSphereVolume))
  (Utilities|FlowControl|Sequence
    (:then_0
      (Components|Sphere|SetSphereRadius _spherevolume (Variables|/Script/Engine.LocalLightComponent|GetAttenuationRadius (Variables|Default|GetPointLightComponent)) true)
      (Transformation|SetWorldScale3D _spherevolume "1.000000,1.000000,1.000000")
      (Rendering|SetVisibility (Variables|Default|GetPointLightComponent) (Variables|CelesLight|GetEnableOriginLight) false))
    (:then_1
      (bind _receiveactors (CallFunction|CelesLightReceiveTrace self (Transformation|GetActorLocation) (Variables|CelesLight|GetCelesLightEffectObjectType) (Variables|CelesLight|GetCelesLightFilterActorTag) (Variables|/Script/Engine.LocalLightComponent|GetAttenuationRadius (Variables|Default|GetPointLightComponent))))
      (for _array_element _receiveactors
        (Utilities|IsValid (Actor|GetComponentbyClass _array_element "/Game/CelesAnimeShader/BP/CelesLight/AC_CelesLightReceive.AC_CelesLightReceive_C")
          (:Is%20Valid
            (Default|RegistLight (Actor|GetComponentbyClass _array_element "/Game/CelesAnimeShader/BP/CelesLight/AC_CelesLightReceive.AC_CelesLightReceive_C") self true)))))
    (:then_2
      (Default|CallOnEditorConstruction))))

(fn GetActor
  (return self))

(fn GetCelesLightData
  (return (Variables|CelesLight|GetCelesLightIntensityMultiply) (Variables|CelesLight|GetCelesLightSmoothStepMin) (Variables|CelesLight|GetCelesLightSmoothStepMax) (Variables|CelesLight|GetCelesLightEffectObjectType) (Variables|CelesLight|GetCelesLightFilterActorTag)))

(fn GetLight
  (return (Variables|Default|GetPointLightComponent)))