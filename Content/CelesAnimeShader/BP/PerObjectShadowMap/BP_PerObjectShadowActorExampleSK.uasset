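; BP_PerObjectShadowActorExampleSK is an example actor that sets up per-object shadow map capture for a skeletal mesh.
; It passes a light target, its SkeletalMesh and a SceneCaptureComponent2D to PerObjectShadowCaptureComp, which handles the capture.
; The construction script initializes the component and updates the shadow map for in-editor preview, while BeginPlay only re-initializes it.
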(event EventBeginPlay
  (Default|InitShadowCapture (Variables|Default|GetPerObjectShadowCaptureComp) (Variables|Default|GetLightTarget) (Variables|Default|GetSkeletalMesh) (Variables|Default|GetSceneCaptureComponent2D)))

(event Collision|EventActorBeginOverlap
  (params (OtherActor :type Actor%20Object%20Reference)))

(fn ConstructionScript
  (bind _perobjectshadowcapturecomp (Variables|Default|GetPerObjectShadowCaptureComp))
  ;[1 1 1] In Editor Update
  (Default|InitShadowCapture _perobjectshadowcapturecomp (Variables|Default|GetLightTarget) (Variables|Default|GetSkeletalMesh) (Variables|Default|GetSceneCaptureComponent2D))
  (Default|UpdateShadowmap _perobjectshadowcapturecomp))