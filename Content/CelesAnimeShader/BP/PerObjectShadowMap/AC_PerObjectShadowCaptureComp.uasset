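; Actor component that renders a per-object depth shadow map for a target mesh along a directional light's direction.
; InitShadowCapture creates dynamic materials and a render target for a supplied SceneCapture2D.
; While the owner is recently rendered, throttled ticks align the capture to the light, box-trace its show-only actors and recapture.
; Each update also feeds hand-built light-view and orthographic projection vectors to the materials, with an optional debug mesh preview.
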(event EventBeginPlay
  (Class|ActorComponent|SetComponentTickInterval (/ 1.0 (Variables|Performance|GetTickTime/s))))

(event EventTick
  (params (DeltaSeconds :type Float%20%28single-precision%29))
  (if (Class|Actor|WasRecentlyRendered (Components|GetOwner) 0.2)
    (CallFunction|UpdateShadowmap)))

(fn InitShadowCapture
  (params (LightTarget :type Actor%20Object%20Reference) (MeshTarget :type Primitive%20Component%20Object%20Reference) (SceneCaptureTarget :type Scene%20Capture%20Component%202D%20Object%20Reference))
  (Utilities|FlowControl|Sequence
    (:then_0
      ;[1 1 1] GetLightTarget
      (Utilities|IsValid LightTarget
        (:Is%20Valid
          (Variables|Private|SetLightTarget LightTarget))
        (:Is%20Not%20Valid
          (bind _outactors (Actor|GetAllActorsOfClass "/Script/Engine.DirectionalLight"))
          (if (Utilities|Array|IsValidIndex _outactors)
            (Variables|Private|SetLightTarget (Utilities|Array|Get(acopy) _outactors))))))
    (:then_1
      ;[1 1 1] Create Dynamic Material Instance
      (bind _output_get (Variables|Private|SetMeshTarget MeshTarget))
      (Utilities|Array|Clear (Variables|Private|GetMIDCache))
      (Utilities|IsValid _output_get
        (:Is%20Valid
          (for _index (range 0 (- (Rendering|Material|GetNumMaterials (Variables|Private|GetMeshTarget)) 1))
            (bind _returnvalue (Rendering|Material|CreateDynamicMaterialInstance (Variables|Private|GetMeshTarget) _index (Rendering|Material|GetMaterial (Variables|Private|GetMeshTarget) _index) "None" :!class /Script/Engine.PrimitiveComponent))
            (Utilities|Array|Add (Variables|Private|GetMIDCache) _returnvalue)))))
    (:then_2
      (Variables|Private|SetSceneCapture SceneCaptureTarget)
      ;[1 1 1] Create Capture + RT
      (CallFunction|RefreshRT))))

(fn CreateSceneCapture
  (if (not (Utilities|IsValid (Variables|Private|GetSceneCapture)))
    (bind _returnvalue (Game|AddComponentbyClass (Components|GetOwner) "/Script/Engine.SceneCaptureComponent2D" false))
    (bind _output_get (Variables|Private|SetSceneCapture _returnvalue))
    (Variables|/Script/Engine.SceneCaptureComponent2D|SetProjectionType _output_get "Orthographic")
    (Variables|/Script/Engine.SceneCaptureComponent2D|SetOrthoWidth _output_get (Variables|Setting|GetCapture_OrthoWidth))
    (Variables|/Script/Engine.SceneCaptureComponent2D|SetPostProcessBlendWeight _output_get 0.0)
    (Variables|/Script/Engine.SceneCaptureComponent|SetbCaptureEveryFrame _output_get false)
    (Variables|/Script/Engine.SceneCaptureComponent|SetCaptureSource _output_get "SCS_SceneDepth")
    (Variables|/Script/Engine.SceneCaptureComponent|SetbCaptureOnMovement _output_get false)))

(fn RefreshRT
  (bind _scenecapture (Variables|Private|GetSceneCapture))
  (bind _rt_size (Variables|Setting|GetRT_Size))
  (Utilities|IsValid (Variables|Private|GetSceneCapture)
    (:Is%20Valid
      (bind _returnvalue (Rendering|CreateRenderTarget2D _rt_size _rt_size "RTF_RGBA16f"))
      (bind _output_get (Variables|Private|SetRTCache _returnvalue))
      (Variables|/Script/Engine.SceneCaptureComponent2D|SetTextureTarget _scenecapture _output_get)
      (Rendering|SceneCapture|CaptureScene _scenecapture :!class /Script/Engine.SceneCaptureComponent2D)
      (for _array_element (Variables|Private|GetMIDCache)
        (Rendering|Material|SetTextureParameterValue _array_element "RT_Depth" _output_get)))))

(fn ClearRT
  (Variables|Private|SetRTCache 0)
  (Variables|/Script/Engine.SceneCaptureComponent2D|SetTextureTarget (Variables|Private|GetSceneCapture) 0))

(fn UpdateShadowmap
  (bind _scenecapture (Variables|Private|GetSceneCapture))
  (bind _scenecapture_2 (Variables|Private|GetSceneCapture))
  (bind _scenecapture_3 (Variables|Private|GetSceneCapture))
  (bind _debugrtmesh (Variables|Private|GetDebugRTMesh))
  (bind _scenecapture_4 (Variables|Private|GetSceneCapture))
  (bind _lighttarget (Variables|Private|GetLightTarget))
  (bind _capture_orthowidth (Variables|Setting|GetCapture_OrthoWidth))
  (bind _returnvalue (Transformation|GetWorldLocation _scenecapture_2))
  (bind _returnvalue_2 (Transformation|GetWorldLocation _scenecapture))
  (bind _returnvalue_3 (Transformation|GetWorldRotation _scenecapture))
  (bind _returnvalue_4 (Transformation|GetActorRotation _lighttarget))
  (bind _returnvalue_5 (Transformation|GetWorldRotation _scenecapture_2))
  (bind _returnvalue_6 (+ _capture_orthowidth 3e+02))
  (bind _orthowidth (Variables|/Script/Engine.SceneCaptureComponent2D|GetOrthoWidth _scenecapture_3))
  (bind _returnvalue_7 (Math|Vector|GetRightVector _returnvalue_5))
  (bind _returnvalue_8 (Math|Vector|GetUpVector _returnvalue_5))
  (bind _returnvalue_9 (Math|Vector|GetForwardVector _returnvalue_5))
  (bind (_x _y _z) (Math|Vector|BreakVector _returnvalue_9))
  (bind (_x_2 _y_2 _z_2) (Math|Vector|BreakVector _returnvalue_7))
  (bind (_x_3 _y_3 _z_3) (Math|Vector|BreakVector _returnvalue_8))
  (if (Math|Boolean|ANDBoolean (Utilities|IsValid (Variables|Private|GetLightTarget)) (Utilities|IsValid (Variables|Private|GetMeshTarget)) (Utilities|IsValid (Variables|Private|GetSceneCapture)))
    (Utilities|FlowControl|Sequence
      (:then_0
        ;[1 1 1] Update Capture Transform
        (Transformation|SetWorldRotation _scenecapture_4 _returnvalue_4 false false)
        (Transformation|SetWorldLocation _scenecapture_4 (+ (Transformation|GetWorldLocation (Variables|Private|GetMeshTarget)) (* (Math|Vector|GetForwardVector _returnvalue_4) -1.0 (Variables|Setting|GetCapture_Length))) false false))
      (:then_1
        (for _array_element (Variables|Private|GetMIDCache)
          (LocalVariables|SettHandleMID _array_element)
          ;[1 1 1] CaptureData+ProjectionData
          (Rendering|Material|SetVectorParameterValue (LocalVariables|GettHandleMID) "CaptureLocation" (Math|Conversions|ToLinearColor(Vector) (Transformation|GetWorldLocation (Variables|Private|GetSceneCapture))) :!class /Script/Engine.MaterialInstanceDynamic)
          (Rendering|Material|SetVectorParameterValue (LocalVariables|GettHandleMID) "LightMatrixX" (Utilities|Struct|MakeLinearColor _x_2 _x_3 _x 0.0) :!class /Script/Engine.MaterialInstanceDynamic)
          (Rendering|Material|SetVectorParameterValue (LocalVariables|GettHandleMID) "LightMatrixY" (Utilities|Struct|MakeLinearColor _y_2 _y_3 _y 0.0) :!class /Script/Engine.MaterialInstanceDynamic)
          (Rendering|Material|SetVectorParameterValue (LocalVariables|GettHandleMID) "LightMatrixZ" (Utilities|Struct|MakeLinearColor _z_2 _z_3 _z 0.0) :!class /Script/Engine.MaterialInstanceDynamic)
          (Rendering|Material|SetVectorParameterValue (LocalVariables|GettHandleMID) "LightMatrixW" (Utilities|Struct|MakeLinearColor (* (Math|Vector|DotProduct _returnvalue _returnvalue_7) -1.0) (* (Math|Vector|DotProduct _returnvalue_8 _returnvalue) -1.0) (* (Math|Vector|DotProduct _returnvalue_9 _returnvalue) -1.0) 1.0) :!class /Script/Engine.MaterialInstanceDynamic)
          (Rendering|Material|SetVectorParameterValue (LocalVariables|GettHandleMID) "ProjectionX" (Utilities|Struct|MakeLinearColor (/ 2.0 _orthowidth) 0.0 0.0 0.0) :!class /Script/Engine.MaterialInstanceDynamic)
          (Rendering|Material|SetVectorParameterValue (LocalVariables|GettHandleMID) "ProjectionY" (Utilities|Struct|MakeLinearColor 0.0 (/ -2.0 _orthowidth) 0.0 0.0) :!class /Script/Engine.MaterialInstanceDynamic)
          (Rendering|Material|SetVectorParameterValue (LocalVariables|GettHandleMID) "ProjectionZ" (Utilities|Struct|MakeLinearColor 0.0 0.0 (/ 1.0 999.900024) 0.0) :!class /Script/Engine.MaterialInstanceDynamic)
          (Rendering|Material|SetVectorParameterValue (LocalVariables|GettHandleMID) "ProjectionW" (Utilities|Struct|MakeLinearColor 0.0 0.0 (/ 1.0 999.900024) 1.0) :!class /Script/Engine.MaterialInstanceDynamic)))
      (:then_2
        ;[1 1 1] Trace ShowOnly Actor
        (Utilities|Array|Clear (Variables|/Script/Engine.SceneCaptureComponent|GetShowOnlyActors (Variables|Private|GetSceneCapture)))
        (bind _outhits (Class|KismetSystemLibrary|BoxTraceMultiforObjects _returnvalue_2 (+ _returnvalue_2 (* (Variables|Setting|GetCapture_Length) 1.0 (Math|Vector|GetForwardVector _returnvalue_3))) (Math|Vector|MakeVector 0.0 _returnvalue_6 _returnvalue_6) _returnvalue_3 (Utilities|Array|MakeArray "ObjectTypeQuery1" "ObjectTypeQuery2" "ObjectTypeQuery3") false 0 "None" true))
        (for _array_element_2 _outhits
          (Utilities|Array|Add (Variables|/Script/Engine.SceneCaptureComponent|GetShowOnlyActors (Variables|Private|GetSceneCapture)) (.HitActor (Collision|BreakHitResult _array_element_2)))))
      (:then_3
        ;[1 1 1] Debug
        (Utilities|IsValid _debugrtmesh
          (:Is%20Valid
            (bind _returnvalue_10 (Rendering|Material|CreateDynamicMaterialInstance _debugrtmesh 0 "/Game/CelesAnimeShader/BP/PerObjectShadowMap/M_DebugRT.M_DebugRT" "None" :!class /Script/Engine.PrimitiveComponent))
            (Rendering|Material|SetTextureParameterValue _returnvalue_10 "RTTarget" (Variables|Private|GetRTCache))
            (Rendering|Material|SetScalarParameterValue _returnvalue_10 "Depth" (Variables|Setting|GetCapture_Length) :!class /Script/Engine.MaterialInstanceDynamic))))
      (:then_4
        (Rendering|SceneCapture|CaptureScene (Variables|Private|GetSceneCapture) :!class /Script/Engine.SceneCaptureComponent2D)))
    (else
      (Development|PrintString "PerObjectShadowmap Error : Has Not Valid Target" true true "(R=1.000000,G=0.000000,B=0.000000,A=1.000000)"))))

(fn SetDebugRT
  (params (SMMeshActor :type Static%20Mesh%20Actor%20Object%20Reference) (MeshComp :type Primitive%20Component%20Object%20Reference))
  (Utilities|IsValid SMMeshActor
    (:Is%20Valid
      (Variables|Private|SetDebugRTMesh (Variables|/Script/Engine.StaticMeshActor|GetStaticMeshComponent SMMeshActor)))
    (:Is%20Not%20Valid
      (Variables|Private|SetDebugRTMesh MeshComp))))