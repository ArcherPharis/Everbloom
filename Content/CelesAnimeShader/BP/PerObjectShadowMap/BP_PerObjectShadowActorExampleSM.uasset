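; Example actor that demonstrates per-object shadow mapping on a static mesh in the CelesAnimeShader content.
; PerObjectShadowCaptureComp is initialized with the Sphere mesh and a SceneCaptureComponent2D as its capture targets.
; The construction script initializes it without a light target and immediately updates the shadow map.
; BeginPlay initializes it again, this time also passing LightTarget.
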(event EventBeginPlay
  (Default|InitShadowCapture (Variables|Default|GetPerObjectShadowCaptureComp) (Variables|Default|GetLightTarget) (Variables|Default|GetSphere) (Variables|Default|GetSceneCaptureComponent2D)))

(fn ConstructionScript
  (bind _perobjectshadowcapturecomp (Variables|Default|GetPerObjectShadowCaptureComp))
  (Default|InitShadowCapture _perobjectshadowcapturecomp 0 (Variables|Default|GetSphere) (Variables|Default|GetSceneCaptureComponent2D))
  (Default|UpdateShadowmap _perobjectshadowcapturecomp))